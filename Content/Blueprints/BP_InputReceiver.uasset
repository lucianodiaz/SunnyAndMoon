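; BP_InputReceiver listens for a player's input and asks the game mode to spawn that player.
; The Start action calls SpawnPlayerMessage on the game mode, passing its PlayerIndex and itself.
; The 2 key makes the same call, but only when PlayerIndex is above zero.
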(event `InputAction|Start`
  (params (Key :type "Key Structure"))
  (:`Pressed`
    (message `/Game/Blueprints/BPI_GameMode.SpawnPlayer` (`GameplayStatics.GetGameMode`) (`self.PlayerIndex`) self)))

(event `Key|Two`
  (params (Key :type "Key Structure"))
  (:`Pressed`
    (if (> (`self.PlayerIndex`) 0)
      (message `/Game/Blueprints/BPI_GameMode.SpawnPlayer` (`GameplayStatics.GetGameMode`) (`self.PlayerIndex`) self))))

(fn `UserConstructionScript`)