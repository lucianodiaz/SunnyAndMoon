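; Map is a Blueprint that switches its front and ground sprite layers between day and night looks.
; Each call to the ChangeDay event alternates through a FlipFlop, applying the night sprites first and the day sprites on the next call.
; A SetSprites helper loops over each group of six sprite components and assigns the matching sprite from the SpriteDay or SpriteNight array.
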(event `ChangeDay`
  (`/Engine/EditorBlueprintResources/StandardMacros.FlipFlop`
    (:`A`
      (`self.SetSprites` (`|MakeArray` (`self.front`) (`self.front3`) (`self.front4`) (`self.front5`) (`self.front2`) (`self.front1`)) (`|GetArrayItem` (`self.SpriteNight`)))
      (`self.SetSprites` (`|MakeArray` (`self.ground2`) (`self.ground1`) (`self.ground3`) (`self.ground4`) (`self.ground5`) (`self.ground6`)) (`|GetArrayItem` (`self.SpriteNight`) 1)))
    (:`B`
      (`self.SetSprites` (`|MakeArray` (`self.front`) (`self.front3`) (`self.front4`) (`self.front5`) (`self.front2`) (`self.front1`)) (`|GetArrayItem` (`self.SpriteDay`)))
      (`self.SetSprites` (`|MakeArray` (`self.ground2`) (`self.ground1`) (`self.ground3`) (`self.ground4`) (`self.ground5`) (`self.ground6`)) (`|GetArrayItem` (`self.SpriteDay`) 1)))))

(fn `SetSprites`
  (params (OldSprite :type "Array of PaperSpriteComponent Object Reference") (NewSprite :type "PaperSprite Object Reference"))
  (for _array_element OldSprite
    (`PaperSpriteComponent.SetSprite` _array_element NewSprite)))

(fn `UserConstructionScript`)