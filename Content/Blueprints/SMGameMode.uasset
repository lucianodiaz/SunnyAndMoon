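; Game mode for a local multiplayer match on a shared camera, with a time limit, a day/night cycle and a two-player score comparison.
; BeginPlay creates local players at tag-indexed PlayerStarts, possessing input receivers that SpawnPlayer later swaps for Player pawns.
; StartGame begins play once enough players join.
; A looping timer uses Delays to count toward GameOver and flip day/night on the map and grass at random intervals.
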(event `self.ReceiveBeginPlay`
  (bind _outactors (`GameplayStatics.GetAllActorsOfClass` "/Game/Blueprints/SM_CameraActor.SM_CameraActor_C"))
  (set `self.Camera` (`|GetArrayItem` _outactors))
  (bind _outactors_2 (`GameplayStatics.GetAllActorsOfClass` "/Game/Blueprints/Map.Map_C"))
  (set `self.Maps` (`|GetArrayItem` _outactors_2))
  (bind _outactors_3 (`GameplayStatics.GetAllActorsOfClass` "/Game/Assets/Miscelaneous/Grass.Grass_C"))
  (set `self.Grasses` _outactors_3)
  (`self.GetPlayerStartPoints`)
  (`self.SpawnInputReceiver`)
  (`KismetSystemLibrary.K2_SetTimer` null "LoopGame" 0.1 true)
  (bind _returnvalue (`|CreateWidget` "/Game/Widget/GameWidget.GameWidget_C"))
  (`UserWidget.AddToViewport` _returnvalue 0))

(event `LoopGame`
  (if (`self.bIsInGame`)
    (`self.CheckGameFinish`)
    (`self.CheckDay`)))

(event `CheckGameFinish`
  (`KismetSystemLibrary.Delay` 1.0)
  (set `self.CurrentTimeGame` (+ (`self.CurrentTimeGame`) 1))
  (if (>= (`self.CurrentTimeGame`) (`self.GameTime`))
    (set `self.GameOver` true)))

(event `CheckDay`
  (if (`self.ChangeDay`)
    (set `self.ChangeDay` false)
    (bind _output_get (set `self.RandomTime` (`KismetMathLibrary.RandomIntegerInRange` 3 10)))
    (`KismetSystemLibrary.Delay` (`KismetMathLibrary.Conv_IntToDouble` _output_get))
    (set `self.ChangeDay` true)
    (`/Game/Blueprints/Map.ChangeDay` (`self.Maps`))
    (for _array_element (`self.Grasses`)
      (`/Game/Assets/Miscelaneous/Grass.DayNight` _array_element))
    (set `self.bIsDay` (not (`self.bIsDay`)))))

(fn `GameStarted`
  (set `self.bIsInGame` true)
  (`/Game/Blueprints/SM_CameraActor.GameStarted` (`self.Camera`) (`self.Players`)))

(fn `GetDay`
  (returns (Day :type Boolean))
  (return (`self.bIsDay`)))

(fn `GetIsInGame`
  (returns (bIsInGame :type Boolean))
  (return (`self.bIsInGame`)))

(fn `GetPlayerStartPoints`
  (bind _outactors (`GameplayStatics.GetAllActorsOfClass` "/Script/Engine.PlayerStart"))
  (set `self.PlayerStartArray` _outactors))

(fn `NameToInt`
  (params (PlayerStart :type "PlayerStart Object Reference"))
  (returns (ReturnValue :type Integer))
  (return (`KismetStringLibrary.Conv_StringToInt` (`KismetStringLibrary.Conv_NameToString` (`PlayerStart.PlayerStartTag` PlayerStart)))))

(fn `RemoveUnusedCameras`
  (bind _outactors (`GameplayStatics.GetAllActorsOfClass` "/Script/Engine.CameraActor"))
  (for _array_element _outactors
    (`self.K2_DestroyActor` _array_element)))

(fn `SpawnInputReceiver`
  (locals (Index :type Integer))
  (bind _returnvalue (`GameplayStatics.GetPlayerController` (`local.Index`)))
  (for (_ _array_index) (`self.PlayerStartArray`)
    (set `local.Index` _array_index)
    (for _array_element (`self.PlayerStartArray`)
      (if (== (`self.NameToInt` _array_element) (`local.Index`))
        (`GameplayStatics.CreatePlayer` -1)
        (bind _returnvalue_2 (`|SpawnActorFromClass` "/Game/Blueprints/BP_InputReceiver.BP_InputReceiver_C" (`self.GetTransform` (`|GetArrayItem` (`self.PlayerStartArray`) (`local.Index`))) "Undefined" "OverrideRootScale" null (`local.Index`) null))
        (`KismetArrayLibrary.Array_AddUnique` (`self.PlayerInputReceiverArray`) _returnvalue_2)
        (`Controller.Possess` _returnvalue _returnvalue_2)
        (`KismetArrayLibrary.Array_AddUnique` (`self.PlayerControllerArray`) _returnvalue)
        (`PlayerController.SetViewTargetWithBlend` (`GameplayStatics.GetPlayerController` (`local.Index`)) (`self.Camera`) 0.0 "VTBlend_Linear" 0.0 false)))
    (`self.RemoveUnusedCameras`)))

(fn `SpawnPlayer`
  (params (CurrentPlayerIndex :type Integer) (InputReceiver :type "/Game/Blueprints/BP_InputReceiver Object Reference"))
  (returns (Return :type Boolean))
  (bind _returnvalue (`|SpawnActorFromClass` "/Game/Blueprints/Player.Player_C" (`self.GetTransform` (`local.InputReceiver`)) "Undefined" "OverrideRootScale" null (`local.CurrentPlayerIndex`) null))
  (`KismetArrayLibrary.Array_Add` (`self.Players`) _returnvalue)
  (`Controller.Possess` (`GameplayStatics.GetPlayerController` (`local.CurrentPlayerIndex`)) _returnvalue)
  (`PlayerController.SetViewTargetWithBlend` (`GameplayStatics.GetPlayerController` (`local.CurrentPlayerIndex`)) (`self.Camera`) 0.0 "VTBlend_Linear" 0.0 false)
  (return false))

(fn `StartGame`
  (if (>= (`KismetArrayLibrary.Array_Length` (`self.Players`)) (`self.MinPlayers`))
    (`self.GameStarted`)
    (return)))

(fn `UserConstructionScript`)

(fn `Winner`
  (returns (Sunny :type Boolean))
  (bind _players (`self.Players`))
  (if (> (`/Game/Blueprints/Player.Puntuacion` (`|GetArrayItem` _players)) (`/Game/Blueprints/Player.Puntuacion` (`|GetArrayItem` _players 1)))
    (return true)
    (else
      (return false))))